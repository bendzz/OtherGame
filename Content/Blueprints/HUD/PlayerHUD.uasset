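; Player HUD Blueprint that draws short-lived text messages on screen.
; HUDsettext replaces the message array, which DrawHUD draws each frame as stacked lines from mid-screen near the left edge, turning black or unset colors white.
; A parallel timer array accumulates delta time per line, and entries older than two seconds are removed from all three arrays inside the draw loop.
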(event `HUD set text`
  (params (NewParam :type "Array of String"))
  (set `self.TextToWrite` NewParam))

(event `self.ReceiveDrawHUD`
  (params (SizeX :type Integer) (SizeY :type Integer))
  (bind _deletetexttimer (`self.DeleteTextTimer`))
  (bind _textcolor (`self.TextColor`))
  (for (_array_element _array_index) (`self.TextToWrite`)
    (bind _item (`KismetArrayLibrary.Array_Get` _textcolor _array_index))
    (if (not (!= (`KismetMathLibrary.Conv_LinearColorToVector` _item) (0.0 0.0 0.0) :`ErrorTolerance` 0.0))
      (`KismetArrayLibrary.Array_Set` _textcolor _array_index (make `Object.LinearColor` 1.0 1.0 1.0 1.0)))
    (`self.DrawText` _array_element _item (`KismetMathLibrary.Conv_IntToDouble` (/ SizeX 8)) (+ (* _array_index 20.0) (`KismetMathLibrary.Conv_IntToDouble` (/ SizeY 2))))
    (bind _returnvalue (+ (`KismetArrayLibrary.Array_Get` _deletetexttimer _array_index) (`GameplayStatics.GetWorldDeltaSeconds`)))
    (`KismetArrayLibrary.Array_Set` _deletetexttimer _array_index _returnvalue true)
    (if (> _returnvalue 2.0)
      (`KismetArrayLibrary.Array_Remove` (`self.TextToWrite`) _array_index)
      (`KismetArrayLibrary.Array_Remove` (`self.DeleteTextTimer`) _array_index)
      (`KismetArrayLibrary.Array_Remove` (`self.TextColor`) _array_index))))

(fn `UserConstructionScript`)