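; Fiesta mode actor that drops potions from the sky over a fixed area of the level.
; Each Tick, while the potion count is below the maximum, it traces downward from random points in a hard-coded box to find a surface.
; It spawns a FoxPotion above the hit location, increments the count and marks the potion unarmed.
; Random potion type assignment is present but disconnected.
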(event `self.ReceiveTick`
  (params (DeltaSeconds :type "Float (single-precision)"))
  (bind _returnvalue (`KismetMathLibrary.RandomPointInBoundingBox` (`KismetMathLibrary.MakeVector` 5500.0 9300.0 12650.0) (`KismetMathLibrary.MakeVector` 7500.0 4700.0 350.0)))
  ;[1 1 1] Drop Potions from Sky
  (if (< (`self.Level Potion Count`) (`self.Max Potion Count`))
    ;;[1 1 1] Get position above ground
    (bind _outhit (`KismetSystemLibrary.LineTraceSingle` _returnvalue (+ _returnvalue (0.0 0.0 -13000.0)) "TraceTypeQuery1"))
    (bind _returnvalue_2 (`|SpawnActorFromClass` "/Game/Blueprints/Items/FoxPotion.FoxPotion_C" (`KismetMathLibrary.MakeTransform` (+ (`.Location` (`GameplayStatics.BreakHitResult` _outhit)) (0.0 0.0 400.0)))))
    (set `self.Level Potion Count` (+ (`self.Level Potion Count`) 1))
    (bind _aspotion (cast `/Game/Blueprints/Items/Potion` _returnvalue_2))
    (set `/Game/Blueprints/Items/Potion.Armed` false _aspotion)))

(event `self.ReceiveBeginPlay`
  ;[1 1 1] Drop Potions from Sky
)

(fn `UserConstructionScript`)