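; TfEffect is a timed transformation effect actor that alters a Victim's body shape.
; BeginPlay spawns a new ABodyShape as TargetBody and prints it.
; Each tick advances State by RatePerSecond and delta time, then passes every TargetBody attribute, scaled by State, to AddAttribute on the Victim's current body shape.
; The actor destroys itself once State reaches one, leaving the spawned shape in place.
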(event `self.ReceiveBeginPlay`
  (`self.Init`))

(event `self.ReceiveTick`
  (params (DeltaSeconds :type "Float (single-precision)"))
  (`self.UpdateState`)
  (`self.Apply TfState`))

(event `UpdateState`
  (set `self.State` (+ (`self.State`) (* (`self.RatePerSecond`) (`GameplayStatics.GetWorldDeltaSeconds`))))
  (if (>= (`self.State`) 1.0)
    (`self.TfFinished`)))

(fn `Apply TfState`
  (for _array_element (`/Game/Blueprints/TFblueprints/aBodyShape.BodyShapeAttributes` (`self.TargetBody`))
    (bind (_userfriendlyname _bodyattributeenum _value) (break `/Game/Blueprints/TFblueprints/BodyAttribute` _array_element))
    (`/Game/Blueprints/TFblueprints/aBodyShape.AddAttribute` (`/Game/MainCharacter/BluePrints/TransformingCharacter.CurrentBodyShape` (`self.Victim`)) (make `/Game/Blueprints/TFblueprints/BodyAttribute` _userfriendlyname _bodyattributeenum (* _value (`self.State`))))))

(fn `Init`
  (bind _returnvalue (`|SpawnActorFromClass` "/Game/Blueprints/TFblueprints/aBodyShape.aBodyShape_C" (`KismetMathLibrary.MakeTransform` (0.0 0.0 0.0)) true))
  (set `self.TargetBody` _returnvalue)
  (`KismetSystemLibrary.PrintString` (`KismetStringLibrary.Conv_ObjectToString` _returnvalue)))

(fn `TfFinished`
  (`self.K2_DestroyActor`))

(fn `UserConstructionScript`)