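; Short-lived blast actor that applies a TFType-selected transformation (gender, dog, fox fur, rubber or cement skin, or reset) to nearby characters.
; After a brief delay, it gathers TFinterface actors within ExplosionRadius, read from a GlobalVariables actor spawned on each loop pass.
; Per-type timelines stream positional float arrays to those characters through ApplyTFMessage, then destroy the actor.
; A parallel Clothing timeline animates shorts, socks and shirt opacity for every type except reset.
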(event `self.ReceiveBeginPlay`
  (bind _tf_type (`self.TF Type`))
  (`KismetSystemLibrary.Delay` 0.2)
  (`self.Get TF Actors in Radius`)
  (`|ExecutionSequence`
    (:`then_0`
      (if (!= _tf_type 2)
        (bind (_direction _shortsheight _sockheight _shirtopacity) (`Timeline|Clothing`)
          (:`Update`
            (for _array_element (`self.Affected Characters`)
              (message `/Game/Blueprints/TFinterface.ApplyTF` _array_element (`|MakeArray` 0.0 0.0 0.0 0.0 0.0 0.0 _shortsheight _sockheight _shirtopacity)))))))
    (:`then_1`
      (switch `int` _tf_type
        (:`0`
          (bind (_direction_2 _maleness) (`Timeline|Timeline_0`)
            (:`Update`
              (for _array_element_2 (`self.Affected Characters`)
                (message `/Game/Blueprints/TFinterface.ApplyTF` _array_element_2 (`|MakeArray` 0.0 _maleness _maleness _maleness 0.0))))
            (:`Finished`
              (`self.K2_DestroyActor`))))
        (:`1`
          (bind (_direction_3 _maleness_2) (`Timeline|Timeline_1`)
            (:`Update`
              (for _array_element_3 (`self.Affected Characters`)
                (message `/Game/Blueprints/TFinterface.ApplyTF` _array_element_3 (`|MakeArray` 0.0 _maleness_2 _maleness_2 _maleness_2 0.0))))
            (:`Finished`
              (`self.K2_DestroyActor`))))
        (:`2`
          (`Timeline|Timeline_2`
            (:`Update`
              (for _array_element_4 (`self.Affected Characters`)
                (message `/Game/Blueprints/TFinterface.ApplyTF` _array_element_4 (`|MakeArray` 1e-08 1e-08 1e-08 1e-08 1e-08 1e-08 0.4 0.8 1.0 1e-13 1e-13 1e-14 :!type "Float (single-precision)"))))
            (:`Finished`
              (`self.K2_DestroyActor`))))
        (:`3`
          (bind (_direction_4 _doggyness) (`Timeline|Timeline_3`)
            (:`Update`
              (for _array_element_5 (`self.Affected Characters`)
                (message `/Game/Blueprints/TFinterface.ApplyTF` _array_element_5 (`|MakeArray` _doggyness 0.0 0.0 0.0 _doggyness _doggyness))))
            (:`Finished`
              (`self.K2_DestroyActor`))))
        (:`4`
          (bind (_direction_5 _rubberskin) (`Timeline|Timeline_4`)
            (:`Update`
              (for _array_element_6 (`self.Affected Characters`)
                (message `/Game/Blueprints/TFinterface.ApplyTF` _array_element_6 (`|MakeArray` 0.0 0.0 0.0 0.0 0.0 0.0 0.0 0.0 0.0 _rubberskin))))
            (:`Finished`
              (`self.K2_DestroyActor`))))
        (:`5`
          (bind (_direction_6 _foxfur) (`Timeline|Timeline_5`)
            (:`Update`
              (for _array_element_7 (`self.Affected Characters`)
                (message `/Game/Blueprints/TFinterface.ApplyTF` _array_element_7 (`|MakeArray` _foxfur 0.0 0.0 0.0 _foxfur 0.0 0.0 0.0 0.0 0.0 _foxfur))))
            (:`Finished`
              (`self.K2_DestroyActor`))))
        (:`6`
          (bind (_direction_7 _cement_skin) (`Timeline|Timeline_6`)
            (:`Update`
              (for _array_element_8 (`self.Affected Characters`)
                (message `/Game/Blueprints/TFinterface.ApplyTF` _array_element_8 (`|MakeArray` 0.0 0.0 0.0 0.0 0.0 0.0 0.0 0.0 0.0 0.0 0.0 _cement_skin))))
            (:`Finished`
              (`self.K2_DestroyActor`))))))))

(fn `Get TF Actors in Radius`
  (bind _outactors (`GameplayStatics.GetAllActorsWithInterface` "/Game/Blueprints/TFinterface.TFinterface_C"))
  (for _array_element _outactors
    (bind _returnvalue (`|SpawnActorFromClass` (`self.Global Variables`) (`KismetMathLibrary.MakeTransform` (0.0 0.0 0.0)) true))
    (bind _asglobal_variables (cast `/Game/Blueprints/GamePlayBlueprints/GlobalVariables` _returnvalue))
    (if (< (`KismetMathLibrary.VSize` (- (`self.K2_GetActorLocation` _array_element) (`self.K2_GetActorLocation`))) (`/Game/Blueprints/GamePlayBlueprints/GlobalVariables.ExplosionRadius` _asglobal_variables))
      (`KismetArrayLibrary.Array_Add` (`self.Affected Characters`) _array_element)
      (message `/Game/Blueprints/TFinterface.InitForTF` _array_element))))

(fn `UserConstructionScript`)