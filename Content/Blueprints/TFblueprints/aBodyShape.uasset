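; aBodyShape is a Blueprint that stores a body shape as an array of attributes keyed by a body attribute enum.
; It offers get, add and delete functions for single attributes, with batch versions that loop over them.
; AddAttribute overwrites a matching entry but still appends afterward.
; GetAttribute never exits its loop early, so it returns the last element alongside the found flag.
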(fn ConstructionScript)

(fn GetAttribute
  (params (BodyAttributeEnum :type EBodyAttributes%20Enum :default "NewEnumerator11"))
  (bind _array_element (Utilities|Array|ForEachLoopwithBreak (Variables|Default|GetBodyShapeAttributes))
    (:LoopBody
      (LocalVariables|SetReturnAttribute _array_element)
      (if (== BodyAttributeEnum (.BodyAttributeEnum (Utilities|Struct|BreakBodyAttribute _array_element)))
        (LocalVariables|SetFound true)))
    (:Completed
      (return (LocalVariables|GetReturnAttribute) (LocalVariables|GetFound)))))

(fn GetAttributes
  (params (BodyAttributeEnums :type Array%20of%20EBodyAttributes%20Enums))
  (bind _array_element (Utilities|Array|ForEachLoopwithBreak BodyAttributeEnums)
    (:LoopBody
      (bind (_bodyattribute _foundattribute) (CallFunction|GetAttribute _array_element))
      (Utilities|Array|Add (LocalVariables|GetReturnAttributes) _bodyattribute)
      (Utilities|Array|Add (LocalVariables|GetFoundAttributes) _foundattribute))
    (:Completed
      (return (LocalVariables|GetReturnAttributes) (LocalVariables|GetFoundAttributes)))))

(fn AddAttribute
  (params (AttributeEnum :type Body%20Attribute%20Structure))
  (bind _bodyshapeattributes (Variables|Default|GetBodyShapeAttributes))
  (bind (_array_element _array_index) (Utilities|Array|ForEachLoopwithBreak (Variables|Default|GetBodyShapeAttributes) :!label _label)
    (:LoopBody
      (if (== (.BodyAttributeEnum (Utilities|Struct|BreakBodyAttribute AttributeEnum)) (.BodyAttributeEnum (Utilities|Struct|BreakBodyAttribute _array_element)))
        (Utilities|FlowControl|Sequence
          (:then_0
            (Utilities|Array|SetArrayElem _bodyshapeattributes _array_index AttributeEnum))
          (:then_1
            (goto _label Break)))))
    (:Completed
      (Utilities|Array|Add _bodyshapeattributes AttributeEnum))))

(fn AddAttributes
  (params (Attributes :type Array%20of%20Body%20Attribute%20Structures))
  (bind _array_element (Utilities|Array|ForEachLoopwithBreak Attributes)
    (:LoopBody
      (CallFunction|AddAttribute _array_element))))

(fn DeleteAttribute
  (params (AttributeEnum :type EBodyAttributes%20Enum :default "NewEnumerator11"))
  (bind _bodyshapeattributes (Variables|Default|GetBodyShapeAttributes))
  (bind (_array_element _array_index) (Utilities|Array|ForEachLoopwithBreak _bodyshapeattributes)
    (:LoopBody
      (if (== (.BodyAttributeEnum (Utilities|Struct|BreakBodyAttribute _array_element)) AttributeEnum)
        (LocalVariables|SetFound true)
        (Utilities|Array|RemoveIndex _bodyshapeattributes _array_index)))
    (:Completed
      (return (LocalVariables|GetFound)))))

(fn DeleteAttributes
  (params (Attributes :type Array%20of%20EBodyAttributes%20Enums))
  (bind _array_element (Utilities|Array|ForEachLoopwithBreak Attributes)
    (:LoopBody
      (bind _foundattribute (CallFunction|DeleteAttribute _array_element))
      (Utilities|Array|Add (LocalVariables|GetFound) _foundattribute))
    (:Completed
      (return (LocalVariables|GetFound)))))