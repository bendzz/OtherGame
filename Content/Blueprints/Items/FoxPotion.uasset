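; Fox potion item Blueprint that gives its potion mesh an orange liquid color.
; On BeginPlay it sets the LiquidColor parameter on PotionMID and applies that material to the first slot of StaticMesh1; the construction script just calls its parent.
; Pour is a debug-print stub.
; A Drink print and a GlobalVariables spawn with an unused color lookup by PotionType are left disconnected and never run.
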(event `self.ReceiveBeginPlay`
  (bind _potion_mid (`self.Potion MID`))
  (`MaterialInstanceDynamic.SetVectorParameterValue` _potion_mid "LiquidColor" (struct :`R` 1.0 :`G` 0.544077 :`A` 1.0))
  (`PrimitiveComponent.SetMaterial` (`self.StaticMesh1`) 0 _potion_mid))

(event `self.Pour`
  (`KismetSystemLibrary.PrintString` "Pour"))

(fn `UserConstructionScript`
  (`parent.UserConstructionScript`))