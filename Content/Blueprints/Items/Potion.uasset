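; Potion item actor offering Drink, Throw and Pour options; Drink spawns a TfEffect on the user, while Throw only prints and Pour is empty.
; On authority, Tick shrinks armed potions and detects impacts on explosion-armed ones through sudden velocity changes.
; An impact spawns a GirlyBoom carrying the PotionType, then destroys the potion.
; Construction creates a dynamic material, but overlap pickup and type-based liquid coloring are disconnected.
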(event `self.Use An Item Option`
  (params (Option :type Integer) (UsingCharacter :type "/Game/MainCharacter/BluePrints/TransformingCharacter Object Reference (by ref)"))
  (switch `int` Option
    (:`0`
      (`self.Drink` UsingCharacter))
    (:`1`
      (`self.Throw`))
    (:`2`
      (`self.Pour`))))

(event `self.CollisionSphere.OnComponentBeginOverlap`
  (params (OtherActor :type "Actor Object Reference") (OtherComp :type "PrimitiveComponent Object Reference") (OtherBodyIndex :type Integer) (bFromSweep :type Boolean) (SweepResult :type "EngineTypes.HitResult Structure (by ref)"))
  ;[1 1 1] Player pickup potion
)

(event `self.ReceiveTick`
  (params (DeltaSeconds :type "Float (single-precision)"))
  (bind _previous_velocity (`self.Previous Velocity`))
  (bind _returnvalue (`SceneComponent.GetComponentVelocity` (`self.StaticMesh1`)))
  (`/Engine/EditorBlueprintResources/ActorMacros.Switch Has Authority`
    (:`Authority`
      (`|ExecutionSequence`
        (:`then_0`
          ;[1 1 1] Make armed potion: Client
          (if (`self.Armed`)
            (`self.SetActorScale3D` (`KismetMathLibrary.MakeVector` 0.5 0.5 0.5))))
        (:`then_1`
          ;[1 1 1] Making armed potion: Server. Check for collision
          (if (`self.Armed to Explode`)
            (if (!= _previous_velocity (0.0 0.0 0.0) :`ErrorTolerance` 0.0)
              (if (> (`KismetMathLibrary.VSize` (- _returnvalue _previous_velocity)) 50.0)
                ;[1 1 1] Collided. Spawn 'explosion'. Despawn potion.
                (bind _returnvalue_2 (`|SpawnActorFromClass` (`self.GirlyBoom`) (`self.GetTransform`)))
                (bind _asgirly_boom (cast `/Game/Blueprints/TFblueprints/GirlyBoom` _returnvalue_2))
                (set `/Game/Blueprints/TFblueprints/GirlyBoom.TF Type` (`self.Potion Type`) _asgirly_boom)
                (`self.K2_DestroyActor`)
                (else
                  (set `self.Previous Velocity` _returnvalue)))
              (else
                (set `self.Previous Velocity` _returnvalue)))))))))

(fn `Drink`
  (params (Character :type "/Game/MainCharacter/BluePrints/TransformingCharacter Object Reference"))
  (`|SpawnActorFromClass` (`self.TfEffect`) (`KismetMathLibrary.MakeTransform` (0.0 0.0 0.0)) true Character)
  (`KismetSystemLibrary.PrintString` "Spawned TfEffect"))

(fn `OnRep_Potion Type`
  ;[1 1 1] Potion type changed
)

(fn `Pour`)

(fn `Throw`
  (`KismetSystemLibrary.PrintString` "Default Throw Function"))

(fn `UserConstructionScript`
  (bind _returnvalue (`KismetMaterialLibrary.CreateDynamicMaterialInstance` "/Game/Blueprints/Items/PotionColor.PotionColor"))
  (set `self.Potion MID` _returnvalue))